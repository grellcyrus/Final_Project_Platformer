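; BP_PhysicsPickup is a colored physics cube that the player can pick up and drop through interact and drop interface events.
; Interacting while empty-handed sets the player's IsHolding flag, turns off cube physics and collision, and snaps the Cube component to the player's Arrow1.
; Dropping calls DetachFromActor and restores collision and physics, without clearing IsHolding.
; The construction script tints the cube with PickupColor through a dynamic material instance.
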(event `/Game/Interfaces/Inter_Interact.INT_Interact`
  (params (PlayerRef :type "/Game/Player/BP_Player Object Reference"))
  (bind _cube (`self.Cube`))
  (if (not (`/Game/Player/BP_Player.isHolding?` PlayerRef))
    (set `/Game/Player/BP_Player.isHolding?` true PlayerRef)
    (`PrimitiveComponent.SetSimulatePhysics` _cube false)
    (`PrimitiveComponent.SetCollisionEnabled` _cube "NoCollision")
    (`SceneComponent.K2_AttachToComponent` (`self.Cube`) (`/Game/Player/BP_Player.Arrow1` PlayerRef) "None" "SnapToTarget" "KeepRelative" "KeepRelative" true)))

(event `/Game/Interfaces/Inter_Interact.INT_Drop`
  (params (PlayerRef :type "/Game/Player/BP_Player Object Reference"))
  (bind _cube (`self.Cube`))
  (`self.K2_DetachFromActor` "KeepWorld" "KeepWorld" "KeepWorld")
  (`PrimitiveComponent.SetCollisionEnabled` _cube "QueryAndPhysics")
  (`PrimitiveComponent.SetSimulatePhysics` _cube true))

(fn `UserConstructionScript`
  (locals (NewLocalVar :type Name :default "None"))
  (bind _returnvalue (`PrimitiveComponent.CreateDynamicMaterialInstance` (`self.Cube`) 0 "/Game/Interactables/MAT_Color.MAT_Color" "None"))
  (bind _output_get (set `self.Color_DMI` _returnvalue))
  (`MaterialInstanceDynamic.SetVectorParameterValue` _output_get "Color" (`self.Pickup_Color`)))