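; Player character with Enhanced Input movement, look and jump, which adds the HUD_TEST widget to the viewport on begin play.
; Interact line-traces from the camera and sends an interface interact message to the hit actor, or a drop message when IsHolding is set.
; Score and damage events update and print Score and Health, and the game quits once Health falls below zero.
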(event `self.ReceiveBeginPlay`
  ; HUD Widget
  (bind _returnvalue (`|CreateWidget` "/Game/UI/HUD_TEST.HUD_TEST_C"))
  (`UserWidget.AddToViewport` _returnvalue 0))

(event `EnhancedInput|/Game/inputs/IA_Interact`
  (params (ActionValue :type Boolean) (ElapsedSeconds :type "Float (double-precision)") (TriggeredSeconds :type "Float (double-precision)") (InputAction :type "InputAction Object Reference" :default "/Game/inputs/IA_Interact.IA_Interact"))
  (bind _camera (`self.Camera`))
  (bind _returnvalue (`SceneComponent.K2_GetComponentLocation` _camera))
  ; Interaction
  (:`Started`
    (if (`self.isHolding?`)
      (message `/Game/Interfaces/Inter_Interact.INT_Drop` (`self.hitObject`) null)
      (set `self.isHolding?` false)
      (else
        (bind (_outhit _returnvalue_2) (`KismetSystemLibrary.LineTraceSingle` :`Start` _returnvalue :`End` (+ _returnvalue (* (`SceneComponent.GetForwardVector` _camera) 800.0)) :`TraceChannel` "TraceTypeQuery1" :`DrawDebugType` "ForDuration"))
        (if _returnvalue_2
          (bind (_bblockinghit _binitialoverlap _time _distance _location _impactpoint _normal _impactnormal _physmat _hitactor) (`GameplayStatics.BreakHitResult` _outhit))
          (set `self.hitObject` _hitactor)
          (message `/Game/Interfaces/Inter_Interact.INT_Interact` _hitactor self))))))

(event `EnhancedInput|/Game/inputs/IA_Movement`
  (params (ActionValue :type "Vector2D Structure") (ElapsedSeconds :type "Float (double-precision)") (TriggeredSeconds :type "Float (double-precision)") (InputAction :type "InputAction Object Reference" :default "/Game/inputs/IA_Movement.IA_Movement"))
  (bind (_returnvalue_roll _returnvalue_pitch _returnvalue_yaw) (`KismetMathLibrary.BreakRotator` (`self.GetControlRotation`)))
  ; Basic Movement
  (:`Triggered`
    (`self.AddMovementInput` (`KismetMathLibrary.GetRightVector` (`KismetMathLibrary.MakeRotator` _returnvalue_roll 0.0 _returnvalue_yaw)) ActionValue_X)
    (`self.AddMovementInput` (`KismetMathLibrary.GetForwardVector` (`KismetMathLibrary.MakeRotator` 0.0 0.0 _returnvalue_yaw)) ActionValue_Y)))

(event `EnhancedInput|/Game/inputs/IA_Look`
  (params (ActionValue :type "Vector2D Structure") (ElapsedSeconds :type "Float (double-precision)") (TriggeredSeconds :type "Float (double-precision)") (InputAction :type "InputAction Object Reference" :default "/Game/inputs/IA_Look.IA_Look"))
  ; Basic Movement
  (:`Triggered`
    (`self.AddControllerYawInput` ActionValue_X)
    (`self.AddControllerPitchInput` ActionValue_Y)))

(event `DropObject`
  ; Interaction
)

(event `EnhancedInput|/Game/inputs/IA_Jump`
  (params (ActionValue :type Boolean) (ElapsedSeconds :type "Float (double-precision)") (TriggeredSeconds :type "Float (double-precision)") (InputAction :type "InputAction Object Reference" :default "/Game/inputs/IA_Jump.IA_Jump"))
  ; Basic Movement
  (:`Triggered`
    (`self.Jump`))
  (:`Canceled`
    (`self.StopJumping`)))

(event `AddScore`
  (params (`Add Amount` :type Integer))
  ; Add Score
  (bind _output_get (set `self.Score` (+ (`self.Score`) `Add Amount`)))
  (`KismetSystemLibrary.PrintString` (`KismetStringLibrary.Conv_IntToString` _output_get)))

(event `self.ReceiveAnyDamage`
  (params (Damage :type "Float (single-precision)") (DamageType :type "DamageType Object Reference") (InstigatedBy :type "Controller Object Reference") (DamageCauser :type "Actor Object Reference"))
  ; Damage Controller
  (bind _output_get (set `self.Health` (- (`self.Health`) Damage)))
  (`KismetSystemLibrary.PrintString` (`KismetStringLibrary.Conv_DoubleToString` _output_get))
  (if (< (`self.Health`) 0.0)
    (`KismetSystemLibrary.QuitGame` null "Quit")))

(fn `UserConstructionScript`)